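; Game mode for the LD55 game, tracking the run timer, six-item win check and finish-camera switch.
; Tick updates the UI and periodically spawns AI at random registered points, meant to avoid the player's nearest, though the minimum-distance search never matches.
; Level actors register themselves here, and registered AI receive the Penta location through their blackboard.
; An HTTP request fetches dreamlo's fastest times and parses them into in-world leaderboard texts.
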(event Custom|ExecuteLeaderboardRequest
  (bind _leaderboardtexts (Variables|Default|GetLeaderboardTexts))
  (bind _result_body (|HttpRequest (Utilities|String|Append "http://dreamlo.com/lb/" (CallFunction|GetReadToken) "/quote-seconds-asc/10") "Get")
    (:On%20Success
      (Variables|Default|SetTempString "")
      (Variables|Default|SetLeaderboardParserIndex 0)
      (for (_array_element _array_index) (Utilities|String|ParseIntoArray (Utilities|String|Replace _result_body ",") "\"")
        (if (== _array_index (Variables|Default|GetLeaderboardParserIndex))
          (Variables|Default|SetTempString _array_element)
          (elif (== _array_index (+ (Variables|Default|GetLeaderboardParserIndex) 2))
            (Development|PrintString (Utilities|String|Append (Variables|Default|GetTempString) ": " (CallFunction|FormatTime (/ (Math|Conversions|ToFloat(Integer) (Math|Conversions|ToInteger(Byte) _array_element)) 1e+01))))
            (Utilities|Array|Add (Variables|Default|GetLeaderboardArray) (Utilities|String|Append (Variables|Default|GetTempString) ": " (CallFunction|FormatTime (/ (Math|Conversions|ToFloat(Integer) (Math|Conversions|ToInteger(Byte) _array_element)) 1e+01))))
            (Variables|Default|SetTempString "")
            (Variables|Default|SetLeaderboardParserIndex (+ (Variables|Default|GetLeaderboardParserIndex) 5)))))
      (for (_array_element_2 _array_index_2) (Variables|Default|GetLeaderboardArray)
        (if (< _array_index_2 (Utilities|Array|Length _leaderboardtexts))
          (Default|UpdateText (Utilities|Array|Get(acopy) _leaderboardtexts _array_index_2) (Utilities|Text|ToText(String) _array_element_2)))))))

(event EventBeginPlay
  (AddComponent|AddAudioComponent false))

(event EventTick
  (params (DeltaSeconds :type Float%20%28single-precision%29))
  (if (not (Variables|Default|GetFinished))
    ;[1 1 1] Timer
    (bind _output_get (Variables|Default|SetTimer (+ DeltaSeconds (Variables|Default|GetTimer))))
    (bind _asbp_player_controller (Utilities|Casting|CastToBP_PlayerController (Game|GetPlayerController 0)))
    (bind _aswbp_default_ui (Utilities|Casting|CastToWBP_DefaultUI (.ui (.CurrentGameState (Default|GetCurrentGameState _asbp_player_controller)))))
    (Default|UpdatefromGameMode _aswbp_default_ui _output_get)
    (bind _output_get_2 (Variables|Default|SetTimeBeforeNewAI (- (Variables|Default|GetTimeBeforeNewAI) DeltaSeconds)))
    (if (<= _output_get_2 0.0)
      (Variables|Default|SetTimeBeforeNewAI 3e+01)
      (CallFunction|SpawnAI))))

(fn ConstructionScript)

(fn RegisterAISpawnPoint
  (params (AISpawnPoint :type BP%20AI%20Spawn%20Point%20Object%20Reference))
  (Utilities|Array|Add (Variables|Default|GetAISpawnPoints) AISpawnPoint))

(fn Finish
  (bind _returnvalue (Game|GetPlayerController 0))
  (bind _finishcamera (Variables|Default|GetFinishCamera))
  (Variables|Default|SetFinished true)
  (bind _asbp_player_controller (Utilities|Casting|CastToBP_PlayerController _returnvalue)
    (:then
      (Default|ChangeGameState _asbp_player_controller "NewEnumerator2"))
    (:CastFailed
      _))
  ;[1 1 1] Disable Player Camera
  (bind _asbp_player_character (Utilities|Casting|CastToBP_PlayerCharacter (Pawn|GetControlledPawn _returnvalue))
    (:then
      (Components|Activation|SetActive (Variables|/Game/LD55/Player/BP_PlayerCharacter.BP_PlayerCharacter_C|GetCamera _asbp_player_character) false false))
    (:CastFailed
      _))
  (Utilities|IsValid _finishcamera
    (:Is%20Valid
      (Components|Activation|SetActive _finishcamera true false)
      (Game|Player|SetViewTargetwithBlend _returnvalue (Components|GetOwner _finishcamera) 0.0 "VTBlend_Linear" 0.0 false))))

(fn AttachandDeactivateFinishCamera
  (params (FinishCamera :type Cine%20Camera%20Component%20Object%20Reference))
  (bind _output_get (Variables|Default|SetFinishCamera FinishCamera))
  (Components|Activation|SetActive _output_get false false))

(fn RegisterAI
  (params (NewAI :type BP%20Base%20AI%20Character%20Object%20Reference))
  (bind _penta (Variables|Default|GetPenta))
  (Utilities|Array|AddUnique (Variables|Default|GetAICharacters) NewAI)
  (Utilities|IsValid _penta
    (:Is%20Valid
      (AI|Components|Blackboard|SetValueasVector (AI|GetBlackboard (Pawn|GetController NewAI)) (Utilities|Name|MakeLiteralName "PentaPos") (Transformation|GetActorLocation _penta)))))

(fn RegisterPenta
  (params (Penta :type BP%20Penta%20Object%20Reference))
  (Variables|Default|SetPenta Penta))

(fn AddItem
  (params (ItemType :type E_Items%20Enum :default "NewEnumerator0"))
  (bind _items (Variables|Default|GetItems))
  (Utilities|Array|AddUnique _items ItemType)
  (if (== 6 (Utilities|Array|Length _items))
    (Development|PrintString "YHEA YOU WON")
    (return true)
    (else
      (return false))))

(fn SpawnAI
  (bind _spawnpoint (CallFunction|GetRandomNotNearestSpawnPoint))
  (Utilities|IsValid _spawnpoint
    (:Is%20Valid
      (Development|PrintString "NewAI")
      (AI|SpawnAIFromClass "/Game/LD55/AI/BP_BaseAICharacter.BP_BaseAICharacter_C" 0 (Transformation|GetActorLocation _spawnpoint) (Transformation|GetActorRotation _spawnpoint) false 0))
    (:Is%20Not%20Valid
      (Development|PrintString "FailToGetAISpawner"))))

(fn GetRandomNotNearestSpawnPoint
  (bind _returnvalue (Game|GetPlayerController 0))
  (bind _aispawnpoints (Variables|Default|GetAISpawnPoints))
  (bind _returnvalue_2 (Utilities|Array|Length _aispawnpoints))
  (bind _returnvalue_3 (Pawn|GetControlledPawn _returnvalue))
  (bind _returnvalue_4 (- _returnvalue_2 1))
  (bind _returnvalue_5 (Math|Random|RandomInteger _returnvalue_4))
  (Utilities|IsValid _returnvalue
    (:Is%20Valid
      (Utilities|IsValid _returnvalue_3
        (:Is%20Valid
          ;[1 1 1] Empty
          (if (Utilities|Array|IsEmpty _aispawnpoints)
            _
            (else
              ;[1 1 1] OnlyOne
              (if (== (Utilities|Array|Length _aispawnpoints) 1)
                (return (Utilities|Array|Get(acopy) _aispawnpoints (Math|Integer|SelectInt (+ _returnvalue_5 1) _returnvalue_5 (>= _returnvalue_5 (LocalVariables|GetMinIndex)))))
                (else
                  (LocalVariables|SetMinIndex -1)
                  (LocalVariables|SetMinDistanceSq -999999.0)
                  (for (_array_element _array_index) _aispawnpoints
                    (if (< (Class|KismetMathLibrary|VectorDistanceSquared (Transformation|GetActorLocation _array_element) (Transformation|GetActorLocation _returnvalue_3)) (LocalVariables|GetMinDistanceSq))
                      (LocalVariables|SetMinDistanceSq (Class|KismetMathLibrary|VectorDistanceSquared (Transformation|GetActorLocation _array_element) (Transformation|GetActorLocation _returnvalue_3)))
                      (LocalVariables|SetMinIndex _array_index)))
                  (return (Utilities|Array|Get(acopy) _aispawnpoints (Math|Integer|SelectInt (+ _returnvalue_5 1) _returnvalue_5 (>= _returnvalue_5 (LocalVariables|GetMinIndex))))))))))
        (:Is%20Not%20Valid
          _)))
    (:Is%20Not%20Valid
      _))
  (return 0))

(fn FillLeaderboard
  (params (Texts :type Array%20of%20BP%20in%20World%20Text%20Object%20References))
  (for _array_element Texts
    (Utilities|Array|AddUnique (Variables|Default|GetLeaderboardTexts) _array_element))
  (CallFunction|ExecuteLeaderboardRequest))

(fn RegisterSacrificeText
  (params (InWorldText :type BP%20in%20World%20Text%20Object%20Reference))
  (bind _output_get (Variables|Default|SetSacrificeText InWorldText))
  (Default|UpdateVisibility _output_get false))

(fn ShowSacrificeText
  (bind _sacrificetext (Variables|Default|GetSacrificeText))
  (Utilities|IsValid _sacrificetext
    (:Is%20Valid
      (Default|UpdateVisibility _sacrificetext true))))