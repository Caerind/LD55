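; BP_PacManPowerSpot is a spawn point that places a BP_PacManPower actor at its own transform on BeginPlay and again after a timed delay.
; Each spawned power receives a reference to the spot through RegisterSpot.
; PrepareTimer, not called within this Blueprint, sets a randomized countdown.
; Tick decrements the timer and respawns the power once it crosses from positive to zero or below.
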(event EventBeginPlay
  (CallFunction|Spawn))

(event EventTick
  (params (DeltaSeconds :type Float%20%28single-precision%29))
  (if (> (Variables|Default|GetTimer) 0.0)
    (bind _output_get (Variables|Default|SetTimer (- (Variables|Default|GetTimer) DeltaSeconds)))
    (if (<= _output_get 0.0)
      (CallFunction|Spawn))
    (else
      (Variables|Default|SetTimer (- (Variables|Default|GetTimer) DeltaSeconds)))))

(fn ConstructionScript)

(fn Spawn
  (bind _returnvalue (Game|SpawnActorfromClass "/Game/LD55/Elements/BP_PacManPower.BP_PacManPower_C" (Math|Transform|MakeTransform (Transformation|GetActorLocation) (Transformation|GetActorRotation) "1.000000,1.000000,1.000000") "AlwaysSpawn" "MultiplyWithRoot" 0 0))
  (Default|RegisterSpot _returnvalue self))

(fn PrepareTimer
  (Variables|Default|SetTimer (Math|Random|RandomFloatinRange 3e+01 45.0)))