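; BP_ItemSpot is a pickup point that holds one item, shown by a static mesh and a point light.
; On BeginPlay, Reset restores the configured start item type, its matching mesh and the light.
; When the player character overlaps a filled spot and its controller holds the default, apparently empty, item type, PickItem passes the item to the controller.
; The spot then adds an audio component, clears its item and mesh, and hides the light.
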(event Collision|EventActorBeginOverlap
  (params (OtherActor :type Actor%20Object%20Reference))
  (if (Utilities|Enum|NotEqual(Enum) (Variables|Default|GetCurrentItemType) "NewEnumerator0")
    (bind _asbp_player_character (Utilities|Casting|CastToBP_PlayerCharacter OtherActor))
    (bind _asbp_player_controller (Utilities|Casting|CastToBP_PlayerController (Pawn|GetController _asbp_player_character)))
    (if (Utilities|Enum|Equal(Enum) (Default|GetItemType _asbp_player_controller) "NewEnumerator0")
      (CallFunction|PickItem _asbp_player_controller))))

(event EventBeginPlay
  (CallFunction|Reset))

(fn ConstructionScript)

(fn Reset
  (bind _startitemtype (Variables|Default|GetStartItemType))
  (Variables|Default|SetCurrentItemType _startitemtype)
  (Components|StaticMesh|SetStaticMesh (Variables|Default|GetStaticMesh) (CallFunction|MeshfromItemType _startitemtype))
  (Rendering|SetVisibility (Variables|Default|GetPointLight) true false))

(fn PickItem
  (params (PlayerController :type BP%20Player%20Controller%20Object%20Reference))
  (Default|SetItemType PlayerController (Variables|Default|GetCurrentItemType))
  (AddComponent|AddAudioComponent false)
  (Variables|Default|SetCurrentItemType "NewEnumerator0")
  (Components|StaticMesh|SetStaticMesh (Variables|Default|GetStaticMesh) 0)
  (Rendering|SetVisibility (Variables|Default|GetPointLight) false false))