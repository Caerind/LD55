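; BP_Penta is a summoning altar actor where the player deposits carried items to complete a sacrifice.
; On overlap it takes the player controller's item, registers it with BP_GameMode, and fills the matching mesh slot, lights its point light and adds audio.
; Once the game mode reports all pieces placed, it shows the sacrifice prompt.
; The first living AI character to overlap then is elevated above it and triggers the game mode's Finish.
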(event EventBeginPlay
  (bind _asbp_game_mode (Utilities|Casting|CastToBP_GameMode (Game|GetGameMode)))
  (Default|RegisterPenta _asbp_game_mode)
  (Rendering|SetVisibility (Variables|Default|GetPointLight1) false false)
  (Rendering|SetVisibility (Variables|Default|GetPointLight2) false false)
  (Rendering|SetVisibility (Variables|Default|GetPointLight3) false false)
  (Rendering|SetVisibility (Variables|Default|GetPointLight6) false false)
  (Rendering|SetVisibility (Variables|Default|GetPointLight5) false false)
  (Rendering|SetVisibility (Variables|Default|GetPointLight4) false false))

(event Collision|EventActorBeginOverlap
  (params (OtherActor :type Actor%20Object%20Reference))
  (bind _asbp_player_character (Utilities|Casting|CastToBP_PlayerCharacter OtherActor)
    (:then
      (bind _asbp_player_controller (Utilities|Casting|CastToBP_PlayerController (Pawn|GetController _asbp_player_character)))
      (if (Utilities|Enum|NotEqual(Enum) (Default|GetItemType _asbp_player_controller) "NewEnumerator0")
        (Development|PrintString (Utilities|String|EnumtoString (Default|GetItemType _asbp_player_controller)))
        (CallFunction|DeposeItem (Default|GetItemType _asbp_player_controller))
        (Default|SetItemType _asbp_player_controller "NewEnumerator0")))
    (:CastFailed
      (bind _asbp_base_aicharacter (Utilities|Casting|CastToBP_BaseAICharacter OtherActor))
      (if (Math|Boolean|ANDBoolean (Variables|Default|GetAllPieces) (not (Variables|Default|GetElevating)) (not (Variables|/Game/LD55/BP_BaseHumanCharacter.BP_BaseHumanCharacter_C|GetIsDead _asbp_base_aicharacter)))
        (Variables|Default|SetElevating true)
        (bind _asbp_game_mode (Utilities|Casting|CastToBP_GameMode (Game|GetGameMode)))
        (Default|Finish _asbp_game_mode)
        (Default|Elevate _asbp_base_aicharacter (+ (Transformation|GetActorLocation) "0.000000,0.000000,150.000000"))))))

(fn ConstructionScript)

(fn DeposeItem
  (params (ItemType :type E_Items%20Enum :default "NewEnumerator0"))
  (bind _mesh (CallFunction|MeshfromItemType ItemType))
  (bind _asbp_game_mode (Utilities|Casting|CastToBP_GameMode (Game|GetGameMode)))
  (Utilities|FlowControl|Sequence
    (:then_0
      ;[1 1 1] Item To GameMode
      (bind _allpieces (Default|AddItem _asbp_game_mode ItemType))
      (bind _output_get (Variables|Default|SetAllPieces _allpieces))
      (if _output_get
        (Default|ShowSacrificeText _asbp_game_mode)))
    (:then_2
      ;[1 1 1] Meshes&Lights
      (AddComponent|AddAudioComponent false)
      (switch Utilities|FlowControl|Switch|SwitchonE_Items ItemType
        (:NewEnumerator1
          (Components|StaticMesh|SetStaticMesh (Variables|Default|GetItem1) _mesh)
          (Rendering|SetVisibility (Variables|Default|GetPointLight1) true false))
        (:NewEnumerator2
          (Components|StaticMesh|SetStaticMesh (Variables|Default|GetItem2) _mesh)
          (Rendering|SetVisibility (Variables|Default|GetPointLight2) true false))
        (:NewEnumerator3
          (Components|StaticMesh|SetStaticMesh (Variables|Default|GetItem3) _mesh)
          (Rendering|SetVisibility (Variables|Default|GetPointLight3) true false))
        (:NewEnumerator4
          (Components|StaticMesh|SetStaticMesh (Variables|Default|GetItem4) _mesh)
          (Rendering|SetVisibility (Variables|Default|GetPointLight4) true false))
        (:NewEnumerator5
          (Components|StaticMesh|SetStaticMesh (Variables|Default|GetItem5) _mesh)
          (Rendering|SetVisibility (Variables|Default|GetPointLight5) true false))
        (:NewEnumerator6
          (Components|StaticMesh|SetStaticMesh (Variables|Default|GetItem6) _mesh)
          (Rendering|SetVisibility (Variables|Default|GetPointLight6) true false))))))