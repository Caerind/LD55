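; BP_InWorldText is an actor that displays text in the world through a widget component hosting WBP_InWorldText.
; BeginPlay pushes its Text variable into the widget and enables Tick only when Follow is set.
; Tick turns the widget to face the first player's controlled pawn, falling back to the controller's location when there is no pawn.
; Functions update the text or toggle the widget's visibility.
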(event EventBeginPlay
  (CallFunction|UpdateText (Variables|Default|GetText))
  (Actor|Tick|SetActorTickEnabled (Variables|Default|GetFollow)))

(event EventTick
  (params (DeltaSeconds :type Float%20%28single-precision%29))
  (bind _returnvalue (Game|GetPlayerController 0))
  (bind _widget (Variables|Default|GetWidget))
  (bind _returnvalue_2 (Pawn|GetControlledPawn _returnvalue))
  (bind _returnvalue_3 (Transformation|GetWorldLocation _widget))
  (Utilities|IsValid _returnvalue
    (:Is%20Valid
      (Utilities|IsValid _returnvalue_2
        (:Is%20Valid
          (Transformation|SetWorldRotation _widget (Math|Rotator|FindLookatRotation _returnvalue_3 (Transformation|GetActorLocation _returnvalue_2)) false false))
        (:Is%20Not%20Valid
          (Transformation|SetWorldRotation _widget (Math|Rotator|FindLookatRotation _returnvalue_3 (Transformation|GetActorLocation _returnvalue)) false false))))))

(fn ConstructionScript)

(fn UpdateText
  (params (Text :type Text))
  (bind _aswbp_in_world_text (Utilities|Casting|CastToWBP_InWorldText (UserInterface|GetWidget (Variables|Default|GetWidget))))
  (Default|SetText _aswbp_in_world_text Text))

(fn UpdateVisibility
  (params (Visibility :type Boolean))
  (Rendering|SetVisibility (Variables|Default|GetWidget) Visibility true))