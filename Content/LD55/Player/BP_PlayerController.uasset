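; Player controller for the LD55 game: handles third-person move and look input, a raycast that spawns impact particles, and the held item's mesh.
; An indexed game-state table pairs each input mapping context with a widget, cursor and pause setting, switching between default, escape and finish screens.
; A timed PacMan mode, counted down on Tick, plays audio and changes the character's light, scale and post-process.
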(event Input|EnhancedActionEvents|EnhancedInputActionIA_Move
  (params (ActionValue :type Vector%202D%20Structure) (ElapsedSeconds :type Float%20%28double-precision%29) (TriggeredSeconds :type Float%20%28double-precision%29) (InputAction :type Input%20Action%20Object%20Reference :default "/Game/LD55/Player/Inputs/IA_Move.IA_Move"))
  ;[1 1 1] Move
  (if (not (Variables|/Game/LD55/BP_BaseHumanCharacter.BP_BaseHumanCharacter_C|GetIsDead (Variables|Default|GetPlayerCharacter)))
    (CallFunction|InputsTPSMovement self (.x ActionValue) (.y ActionValue))))

(event Input|EnhancedActionEvents|EnhancedInputActionIA_Look
  (params (ActionValue :type Vector%202D%20Structure) (ElapsedSeconds :type Float%20%28double-precision%29) (TriggeredSeconds :type Float%20%28double-precision%29) (InputAction :type Input%20Action%20Object%20Reference :default "/Game/LD55/Player/Inputs/IA_Look.IA_Look"))
  ;[1 1 1] Look
  (if (not (Variables|/Game/LD55/BP_BaseHumanCharacter.BP_BaseHumanCharacter_C|GetIsDead (Variables|Default|GetPlayerCharacter)))
    (bind _asbp_game_instance (Utilities|Casting|CastToBP_GameInstance (Game|GetGameInstance)))
    (CallFunction|InputsTPSLook self (.x ActionValue) (.y ActionValue) (Variables|/Game/LD55/BP_GameInstance.BP_GameInstance_C|GetInvertLookAxisY _asbp_game_instance))))

(event Input|EnhancedActionEvents|EnhancedInputActionIA_Raycast
  (params (ActionValue :type Boolean) (ElapsedSeconds :type Float%20%28double-precision%29) (TriggeredSeconds :type Float%20%28double-precision%29) (InputAction :type Input%20Action%20Object%20Reference :default "/Game/LD55/Player/Inputs/IA_Raycast.IA_Raycast"))
  (bind (_location _rotation) (Pawn|GetPlayerViewPoint))
  (:Completed
    (if (not (Variables|/Game/LD55/BP_BaseHumanCharacter.BP_BaseHumanCharacter_C|GetIsDead (Variables|Default|GetPlayerCharacter)))
      (bind (_outhit _returnvalue) (Collision|LineTraceByChannel (+ _location (Math|Vector|MakeVector 0.0 0.0 5e+01)) (+ _location (* (Math|Vector|GetForwardVector _rotation) 1e+04)) "TraceTypeQuery1" false 0 "None"))
      (if _returnvalue
        (Game|SpawnActorfromClass "/Game/LD55/Elements/BP_RaycastParticles.BP_RaycastParticles_C" (Math|Transform|MakeTransform (.location _outhit) (Math|Rotator|CombineRotators (Class|KismetMathLibrary|QuatRotator (Math|Conversions|ToQuaternion(Rotator) (.impactnormal _outhit))) "-90.000000,0.000000,0.000000") "1.000000,1.000000,1.000000") "AlwaysSpawn" "MultiplyWithRoot" self 0)))))

(event Input|EnhancedActionEvents|EnhancedInputActionIA_Escape
  (params (ActionValue :type Boolean) (ElapsedSeconds :type Float%20%28double-precision%29) (TriggeredSeconds :type Float%20%28double-precision%29) (InputAction :type Input%20Action%20Object%20Reference :default "/Game/LD55/Player/Inputs/IA_Escape.IA_Escape"))
  ;[1 1 1] Escape
  (:Completed
    (if (== (Variables|Default|GetCurrentPlayerGameStateIndex) (Math|Conversions|ToInteger(Byte) (Utilities|Enum|LiteralenumE_PlayerGameState "NewEnumerator1")))
      (CallFunction|ChangeGameState (Variables|Default|GetPreviousPlayerGameState))
      (else
        (CallFunction|ChangeGameState "NewEnumerator1")))))

(event EventBeginPlay
  (bind _asbp_player_character (Utilities|Casting|CastToBP_PlayerCharacter (Pawn|GetControlledPawn)))
  (bind _output_get (Variables|Default|SetPlayerCharacter _asbp_player_character))
  (Variables|/Game/LD55/Player/BP_PlayerCharacter.BP_PlayerCharacter_C|SetPlayerController _output_get self)
  (CallFunction|InitGameStates)
  (CallFunction|ChangePacManMode false))

(event EventTick
  (params (DeltaSeconds :type Float%20%28single-precision%29))
  ;[1 1 1] Update PacMan
  (if (Variables|Default|GetPacManMode)
    (bind _output_get (Variables|Default|SetPacManModeTimer (- (Variables|Default|GetPacManModeTimer) DeltaSeconds)))
    (if (<= _output_get 0.0)
      (CallFunction|ChangePacManMode false))))

(fn ConstructionScript)

(fn InitGameStates
  (bind _gamestates (Variables|Default|GetGameStates))
  (bind _returnvalue (Game|ConstructObjectfromClass "/Game/LD55/UI/WBP_DefaultUI.WBP_DefaultUI_C"))
  (Utilities|Array|Add _gamestates (Utilities|Struct|MakeBS_PlayerGameState "NewEnumerator0" "/Game/LD55/Player/Inputs/IMC_Default.IMC_Default" _returnvalue false false))
  (bind _returnvalue_2 (Game|ConstructObjectfromClass "/Game/LD55/UI/WBP_EscapeUI.WBP_EscapeUI_C"))
  (Utilities|Array|Add _gamestates (Utilities|Struct|MakeBS_PlayerGameState "NewEnumerator1" "/Game/LD55/Player/Inputs/IMC_Escape.IMC_Escape" _returnvalue_2 true true))
  (bind _returnvalue_3 (Game|ConstructObjectfromClass "/Game/LD55/UI/WBP_FinishUI.WBP_FinishUI_C"))
  (Utilities|Array|Add _gamestates (Utilities|Struct|MakeBS_PlayerGameState "NewEnumerator1" "/Game/LD55/Player/Inputs/IMC_Finish.IMC_Finish" _returnvalue_3 true false))
  ;[1 1 1] Start "Default"
  (Variables|Default|SetPreviousPlayerGameState "NewEnumerator0")
  (CallFunction|ChangeGameState "NewEnumerator0"))

(fn ChangeGameState
  (params (NewPlayerGameState :type E_PlayerGameState%20Enum :default "NewEnumerator0"))
  (bind _returnvalue (Math|Conversions|ToInteger(Byte) NewPlayerGameState))
  (bind (_currentgamestate _valid) (CallFunction|GetCurrentGameState))
  (bind (_currentgamestate_2 _valid_2) (CallFunction|GetCurrentGameState))
  ;[1 1 1] Early out if we already are in this state
  (if (== (Variables|Default|GetCurrentPlayerGameStateIndex) _returnvalue)
    (return)
    (else
      (if _valid
        ;[1 1 1] Clean previous state if any
        (Variables|Default|SetPreviousPlayerGameState (.gamestate _currentgamestate))
        (Utilities|IsValid (.imc _currentgamestate)
          (:Is%20Valid
            (Input|RemoveMappingContext (PlayerController|LocalPlayerSubsystems|GetEnhancedInputLocalPlayerSubsystem) (.imc _currentgamestate) "(bIgnoreAllPressedKeysUntilRelease=True,bForceImmediately=False,bNotifyUserSettings=False)"))
          (:Is%20Not%20Valid
            _))
        (Utilities|IsValid (.ui _currentgamestate)
          (:Is%20Valid
            (Default|OnDeactivate (.ui _currentgamestate) (.gamestate _currentgamestate))
            (Widget|RemovefromParent (.ui _currentgamestate)))
          (:Is%20Not%20Valid
            _)))
      (Variables|Default|SetCurrentPlayerGameStateIndex _returnvalue)
      (if _valid_2
        ;[1 1 1] Apply new state
        (Utilities|IsValid (.imc _currentgamestate_2)
          (:Is%20Valid
            (Input|AddMappingContext (PlayerController|LocalPlayerSubsystems|GetEnhancedInputLocalPlayerSubsystem) (.imc _currentgamestate_2) 0 "(bIgnoreAllPressedKeysUntilRelease=True,bForceImmediately=False,bNotifyUserSettings=False)"))
          (:Is%20Not%20Valid
            _))
        (Utilities|IsValid (.ui _currentgamestate_2)
          (:Is%20Valid
            (Default|OnActivate (.ui _currentgamestate_2) (Variables|Default|GetPreviousPlayerGameState))
            (UserInterface|Viewport|AddtoViewport (.ui _currentgamestate_2) 0))
          (:Is%20Not%20Valid
            _))
        (Variables|Default|SetbShowMouseCursor (.mousecursor _currentgamestate_2))
        (Game|SetGamePaused (.pausegame _currentgamestate_2))))))

(fn GetCurrentGameState
  (bind _currentplayergamestateindex (Variables|Default|GetCurrentPlayerGameStateIndex))
  (if (and (> (Utilities|Array|Length (Variables|Default|GetGameStates)) _currentplayergamestateindex) (>= _currentplayergamestateindex 0))
    (return (Utilities|Array|Get(acopy) (Variables|Default|GetGameStates) (Variables|Default|GetCurrentPlayerGameStateIndex)) true)
    (else
      (return "" false))))

(fn ChangePacManMode
  (params (Activate :type Boolean))
  (bind _playercharacter (Variables|Default|GetPlayerCharacter))
  (bind _pointlight (Variables|/Game/LD55/Player/BP_PlayerCharacter.BP_PlayerCharacter_C|GetPointLight _playercharacter))
  (bind _output_get (Variables|Default|SetPacManMode Activate))
  (if _output_get
    (Utilities|IsValid (Variables|Default|GetPacman%20Sound)
      (:Is%20Valid
        (Audio|Components|Audio|Stop (Variables|Default|GetPacman%20Sound))
        (Variables|Default|SetPacman%20Sound 0))
      (:Is%20Not%20Valid
        _))
    (bind _returnvalue (AddComponent|AddAudioComponent false))
    (Variables|Default|SetPacman%20Sound _returnvalue)
    (Variables|Default|SetPacManModeTimer 1e+01)
    (else
      (Utilities|IsValid (Variables|Default|GetPacman%20Sound)
        (:Is%20Valid
          (Audio|Components|Audio|Stop (Variables|Default|GetPacman%20Sound))
          (Variables|Default|SetPacman%20Sound 0))
        (:Is%20Not%20Valid
          _))
      (Variables|Default|SetPacManModeTimer -1.0)))
  (Utilities|IsValid _playercharacter
    (:Is%20Valid
      (Rendering|Lighting|SetAttenuationRadius _pointlight (Math|Float|SelectFloat 2e+03 4e+02 (>= (Variables|Default|GetPacManModeTimer) 0.0)))
      (Rendering|Components|Light|SetIntensity _pointlight (Math|Float|SelectFloat 1e+03 1e+02 (>= (Variables|Default|GetPacManModeTimer) 0.0)))
      (Rendering|Components|Light|SetLightColor _pointlight (Math|Color|SelectColor "(R=0.000000,G=1.000000,B=0.108257,A=1.000000)" "(R=0.000000,G=0.223844,B=1.000000,A=1.000000)" (>= (Variables|Default|GetPacManModeTimer) 0.0)) true)
      (Transformation|SetActorScale3D _playercharacter (Math|Vector|SelectVector "1.500000,1.500000,1.500000" "1.000000,1.000000,1.000000" (>= (Variables|Default|GetPacManModeTimer) 0.0)))
      (Rendering|SetVisibility (Variables|/Game/LD55/Player/BP_PlayerCharacter.BP_PlayerCharacter_C|GetPostProcess _playercharacter) (>= (Variables|Default|GetPacManModeTimer) 0.0) false))))

(fn IsinPacManMode
  (return (Variables|Default|GetPacManMode)))

(fn SetItemType
  (params (ItemType :type E_Items%20Enum :default "NewEnumerator0"))
  (bind _output_get (Variables|Default|SetItemType ItemType))
  (Components|StaticMesh|SetStaticMesh (Variables|/Game/LD55/BP_BaseHumanCharacter.BP_BaseHumanCharacter_C|GetObjetActif (Variables|Default|GetPlayerCharacter)) (CallFunction|MeshfromItemType _output_get)))

(fn GetItemType
  (return (Variables|Default|GetItemType)))