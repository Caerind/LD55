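; Player character Blueprint that can kill AI characters on contact while its controller is in Pac-Man mode.
; On BeginPlay it randomly picks one of two skeletal meshes, a ghost or a tormented soul, and Tick runs PlayerWalking every frame.
; KillSphere overlaps check the mode, then hide the AI's spotlight, unpossess its AI controller and call Kill on it.
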(event OnComponentBeginOverlap(KillSphere)
  (params (OverlappedComponent :type Primitive%20Component%20Object%20Reference) (OtherActor :type Actor%20Object%20Reference) (OtherComp :type Primitive%20Component%20Object%20Reference) (OtherBodyIndex :type Integer) (bFromSweep :type Boolean) (SweepResult :type Hit%20Result%20Structure%20%28by%20ref%29))
  (bind _playercontroller (Variables|Default|GetPlayerController))
  (Utilities|IsValid _playercontroller
    (:Is%20Valid
      (if (Default|IsinPacManMode _playercontroller)
        (bind _asbp_base_aicharacter (Utilities|Casting|CastToBP_BaseAICharacter OtherActor))
        (Rendering|SetVisibility (Variables|/Game/LD55/AI/BP_BaseAICharacter.BP_BaseAICharacter_C|GetSpotLight _asbp_base_aicharacter) false false)
        (Utilities|IsValid (AI|GetAIController _asbp_base_aicharacter)
          (:Is%20Valid
            (Pawn|UnPossess (AI|GetAIController _asbp_base_aicharacter)))
          (:Is%20Not%20Valid
            _))
        (Default|Kill _asbp_base_aicharacter false)))))

(event EventBeginPlay
  (bind _mesh (Variables|Character|GetMesh))
  (if (Math|Random|RandomBool)
    (Components|SkeletalMesh|SetSkeletalMeshAsset _mesh "/Game/PolygonDungeons/Meshes/Characters/SK_Character_Ghost_01.SK_Character_Ghost_01")
    (else
      (Components|SkeletalMesh|SetSkeletalMeshAsset _mesh "/Game/PolygonDungeons/Meshes/Characters/SK_Character_Tormented_Soul.SK_Character_Tormented_Soul"))))

(event EventTick
  (params (DeltaSeconds :type Float%20%28single-precision%29))
  (CallFunction|PlayerWalking self))

(fn ConstructionScript
  (|CallParentFunction))