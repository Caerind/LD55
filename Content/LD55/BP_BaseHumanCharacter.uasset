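; Base human character Blueprint for the LD55 game that provides shared health and death handling.
; Health resets to its maximum on BeginPlay, and a getter returns it as a clamped, divide-safe percentage.
; Kill flags the character dead, then either destroys it instantly or enables physics on mesh and capsule, sets a delayed despawn via lifespan, and adds particle and audio components.
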(event EventBeginPlay
  (CallFunction|ResetStats))

(fn ConstructionScript)

(fn ResetStats
  (Variables|Default|SetHealth (Variables|Default|GetHealthMax)))

(fn GetHealthPercent
  (return (Math|Float|Clamp(Float) (Math|Float|SafeDivide (Variables|Default|GetHealth) (Variables|Default|GetHealthMax)))))

(fn Kill
  (params (Instant :type Boolean))
  (bind _mesh (Variables|Character|GetMesh))
  (Variables|Default|SetIsDead true)
  (if Instant
    (Actor|DestroyActor)
    (else
      (Physics|SetSimulatePhysics _mesh true)
      (Collision|SetCollisionEnabled _mesh "QueryAndPhysics")
      (Physics|SetSimulatePhysics (Variables|Collision|GetCapsuleComponent) true)
      (Actor|SetLifeSpan 2.4e+02)
      (AddComponent|AddParticleSystemComponent false)
      (AddComponent|AddAudioComponent false))))