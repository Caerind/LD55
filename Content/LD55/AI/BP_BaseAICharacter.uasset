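; Base AI character that kills the player when its punch detector overlaps their capsule, unless Pac-Man mode is active.
; A kill triggers a random salsa or swing animation, then reloads the map after a delay unless the game has finished.
; It registers with BP_GameMode after spawn and supports resetting to its start transform.
; Elevate teleports it, disables gravity and AI control, then Tick raises it with particles, otherwise handling randomly timed walking sounds.
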(event OnComponentBeginOverlap(PunchDetector)
  (params (OverlappedComponent :type Primitive%20Component%20Object%20Reference) (OtherActor :type Actor%20Object%20Reference) (OtherComp :type Primitive%20Component%20Object%20Reference) (OtherBodyIndex :type Integer) (bFromSweep :type Boolean) (SweepResult :type Hit%20Result%20Structure%20%28by%20ref%29))
  (bind _mesh (Variables|Character|GetMesh))
  (if (not (Variables|Default|GetIsDead))
    (bind _asbp_player_character (Utilities|Casting|CastToBP_PlayerCharacter OtherActor))
    (if (and (not (Default|IsinPacManMode (Variables|/Game/LD55/Player/BP_PlayerCharacter.BP_PlayerCharacter_C|GetPlayerController _asbp_player_character))) (== (Variables|/Script/Engine.Character|GetCapsuleComponent _asbp_player_character) OtherComp))
      (Pawn|UnPossess (Variables|/Game/LD55/Player/BP_PlayerCharacter.BP_PlayerCharacter_C|GetPlayerController _asbp_player_character))
      (Default|Kill _asbp_player_character false)
      (if (Math|Random|RandomBool)
        (Components|Animation|PlayAnimation _mesh "/Game/Characters/MixamoSyntyDungeon/Animations/AM_Salsa.AM_Salsa" false)
        (else
          (Components|Animation|PlayAnimation _mesh "/Game/Characters/MixamoSyntyDungeon/Animations/AM_Swing.AM_Swing" false)))
      (bind _asbp_game_mode (Utilities|Casting|CastToBP_GameMode (Game|GetGameMode))
        (:then
          (if (not (Variables|/Game/LD55/BP_GameMode.BP_GameMode_C|GetFinished _asbp_game_mode))
            (Utilities|FlowControl|Delay 5.0 :!label _label)
            (Game|OpenLevel(byObjectReference) "/Game/LD55/Maps/GameMap/GameMap.GameMap")))
        (:CastFailed
          (goto _label))))))

(event EventBeginPlay
  (|CallParentFunction)
  (Variables|Default|SetInitialLocation (Transformation|GetActorLocation))
  (Variables|Default|SetInitialRotation (Transformation|GetActorRotation))
  ;[1 1 1] Register after pentagram
  (Utilities|FlowControl|Delay 0.5)
  (bind _asbp_game_mode (Utilities|Casting|CastToBP_GameMode (Game|GetGameMode)))
  (Default|RegisterAI _asbp_game_mode self))

(event EventTick
  (params (DeltaSeconds :type Float%20%28single-precision%29))
  (bind _output_get (Variables|Default|SetElevatingTime (- (Variables|Default|GetElevatingTime) DeltaSeconds)))
  (if (>= _output_get 0.0)
    (Transformation|AddActorWorldOffset (Math|Vector|MakeVector 0.0 0.0 (* DeltaSeconds (Variables|Default|GetElevatingSpeed))) false true)
    (AddComponent|AddParticleSystemComponent false (Math|Transform|MakeTransform "0, 0, 0" (Math|Random|RandomRotator false) "3.000000,3.000000,3.000000"))
    (else
      (if (Variables|Default|GetStartedElevate)
        (Variables|Default|SetStartedElevate false)
        (AddComponent|AddAudioComponent false))
      (bind _output_get_2 (Variables|Default|SetWalkingSoundTimer (- (Variables|Default|GetWalkingSoundTimer) DeltaSeconds)))
      (if (and (>= 1.0 _output_get_2) (>= (Math|Vector|VectorLengthSquared (Variables|/Script/Engine.MovementComponent|GetVelocity (Variables|Character|GetCharacterMovement))) 1e+03))
        (if (not (Variables|Default|GetIsDead))
          (AddComponent|AddAudioComponent false)
          (Variables|Default|SetWalkingSoundTimer (Math|Random|RandomFloatinRange 0.0 2.0)))))))

(fn ConstructionScript
  (|CallParentFunction))

(fn Elevate
  (params (Location :type Vector))
  (bind _returnvalue (Pawn|GetController))
  (bind _self self)
  (bind _mesh (Variables|Character|GetMesh))
  (bind _returnvalue_2 (AI|GetAIController _self))
  (Transformation|SetActorLocation Location false false)
  (Actor|Tick|SetActorTickEnabled true)
  (Components|Animation|SetAnimationMode _mesh "AnimationCustomMode" true)
  (Physics|SetEnableGravity _mesh false)
  (Physics|SetEnableGravity (Variables|Default|GetCapsuleComponent) false)
  (Variables|/Script/Engine.CharacterMovementComponent|SetGravityScale (Variables|Character|GetCharacterMovement) 0.0)
  (Variables|Default|SetElevatingTime (Variables|Default|GetElevatingTimeMax))
  (Variables|Default|SetStartedElevate true)
  (AddComponent|AddAudioComponent false)
  (Utilities|IsValid _returnvalue
    (:Is%20Valid
      (Pawn|UnPossess _returnvalue))
    (:Is%20Not%20Valid
      _))
  (Utilities|IsValid _returnvalue_2
    (:Is%20Valid
      (Pawn|UnPossess _returnvalue_2))))

(fn Reset
  (Transformation|SetActorLocationAndRotation (Variables|Default|GetInitialLocation) (Variables|Default|GetInitialRotation) false true))